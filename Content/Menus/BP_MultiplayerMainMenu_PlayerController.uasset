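; Player controller for the multiplayer main menu that brings up the menu UI when play begins.
; BeginPlay calls CreateMainMenu, which, if IsMainMenuMapOpen is true, creates W_Main_Menu for player 0 and adds it to the viewport.
; It then switches input to UI-only focused on the widget and shows the mouse cursor.
; MainMenuRef is set to None rather than to the new widget.
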(event `self.ReceiveBeginPlay`
  (`|ExecutionSequence`
    (:`then_0`
      (`self.CreateMainMenu`))))

(event `CreateMainMenu`
  (bind _returnvalue (`GameplayStatics.GetPlayerController` 0))
  (if (`self.IsMainMenuMapOpen?`)
    (bind _returnvalue_2 (`|CreateWidget` "/Game/Menus/W_Main_Menu.W_Main_Menu_C" _returnvalue))
    (set `self.MainMenuRef` null)
    (`UserWidget.AddToViewport` _returnvalue_2 0)
    (`WidgetBlueprintLibrary.SetInputMode_UIOnlyEx` _returnvalue _returnvalue_2)
    (set `PlayerController.bShowMouseCursor` true _returnvalue)))

(fn `UserConstructionScript`)