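; B_CheckBlockLines detects and clears completed rows in what appears to be a falling-block game, on a board whose width scales with NumPlayers.
; CheckLines sweeps each row with a horizontal multi line trace against WorldStatic objects.
; A row with enough hits spawns explosions and destroys its blocks, then calls Drop on every B_SingleBlock above it.
; DroppedLines offsets later trace heights to account for cleared rows.
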(event `SpawnEmitter`
  (params (Location :type "Vector Structure"))
  (`GameplayStatics.SpawnEmitterAtLocation` "/Game/StarterContent/Particles/P_Explosion.P_Explosion" Location (struct) (0.5 0.5 0.5)))

(fn `CheckLines`
  (for _index (range (+ (`self.Height`) 1))
    (bind _output_get (set `self.CutoffLineZ` (`KismetMathLibrary.Conv_IntToDouble` (+ (* (- _index (`self.DroppedLines`)) 50) 100))))
    (bind (_outhits _returnvalue) (`KismetSystemLibrary.LineTraceMultiForObjects` :`Start` (`KismetMathLibrary.MakeVector` 0.0 0.0 _output_get) :`End` (`KismetMathLibrary.MakeVector` (`KismetMathLibrary.Conv_IntToDouble` (- (* (`self.NumPlayers`) 10 50) 50)) 0.0 _output_get) :`ObjectTypes` (`|MakeArray` "ObjectTypeQuery1" :!type "EObjectTypeQuery Enum") :`DrawDebugType` "ForDuration"))
    (if _returnvalue
      (if (>= (`KismetArrayLibrary.Array_Length` _outhits) (* (`self.NumPlayers`) 10))
        (for _array_element _outhits
          (bind (_bblockinghit _binitialoverlap _time _distance _location _impactpoint _normal _impactnormal _physmat _hitactor) (`GameplayStatics.BreakHitResult` _array_element))
          (`self.SpawnEmitter` (`self.K2_GetActorLocation` _hitactor))
          (`self.K2_DestroyActor` _hitactor))
        (bind _outactors (`GameplayStatics.GetAllActorsOfClass` "/Game/Blueprints/B_SingleBlock.B_SingleBlock_C"))
        (for _array_element_2 _outactors
          (bind (_returnvalue_x _returnvalue_y _returnvalue_z) (`KismetMathLibrary.BreakVector` (`self.K2_GetActorLocation` _array_element_2)))
          (if (> _returnvalue_z (`self.CutoffLineZ`))
            (`/Game/Blueprints/B_SingleBlock.Drop` _array_element_2)))
        (`/Engine/EditorBlueprintResources/StandardMacros.IncrementInt` (`self.DroppedLines`))))))

(fn `UserConstructionScript`)