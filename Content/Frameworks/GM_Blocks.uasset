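; Game mode for a multiplayer falling-block game that builds the playfield and seats players up to a maximum count.
; BeginPlay spawns the line checker, walls and floor, mostly sized by MaxPlayerCount.
; Each new player possesses a falling-block pawn offset along X and linked to the shared line checker.
; A full lobby triggers StartPlay after a delay; later joiners only get their name printed.
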(event `self.ReceiveBeginPlay`
  (bind _maxplayercount (`self.MaxPlayerCount`))
  ;[1 1 1] Создание Блупринта проверки линий
  (bind _returnvalue (`|SpawnActorFromClass` "/Game/Blueprints/B_CheckBlockLines.B_CheckBlockLines_C" (`KismetMathLibrary.MakeTransform` (0.0 0.0 0.0)) "AlwaysSpawn" "MultiplyWithRoot" null (`self.MaxPlayerCount`) null))
  (set `self.CheckBlocks` _returnvalue)
  ;[1 1 1] Создание стен
  (`|SpawnActorFromClass` "/Game/Blueprints/B_Walls.B_Walls_C" (`KismetMathLibrary.MakeTransform` (0.0 0.0 0.0)) "AlwaysSpawn" "MultiplyWithRoot" null _maxplayercount null)
  ;[1 1 1] Создание пола
  (`|SpawnActorFromClass` "/Game/Blueprints/BP_Floor.BP_Floor_C" (`KismetMathLibrary.MakeTransform` (150.0 0.0 60.0)) "AdjustIfPossibleButAlwaysSpawn" "MultiplyWithRoot" null _maxplayercount null))

(event `self.HandleStartingNewPlayer`
  (params (NewPlayer :type "PlayerController Object Reference"))
  ;[1 1 1] Создание и вселение в персонажа при подключении игрока
  (`KismetSystemLibrary.Delay` 0.1)
  (if (== (`self.CurrentPleyerCount`) (`self.MaxPlayerCount`))
    (`KismetSystemLibrary.PrintString` (`KismetSystemLibrary.GetDisplayName` NewPlayer) true true (struct :`R` 1.0 :`G` 0.278251 :`B` 0.238443 :`A` 1.0))
    (else
      (bind _returnvalue (`|SpawnActorFromClass` "/Game/Blueprints/P_FallenBlock.P_FallenBlock_C" (`KismetMathLibrary.MakeTransform` (`KismetMathLibrary.MakeVector` (`KismetMathLibrary.Conv_IntToDouble` (+ (* (`self.CurrentPleyerCount`) 500) 200)) 0.0 1000.0)) "AlwaysSpawn" "MultiplyWithRoot" null (`self.CheckBlocks`) null))
      (`/Engine/EditorBlueprintResources/StandardMacros.IncrementInt` (`self.CurrentPleyerCount`)
        (:`  `
          (`Controller.Possess` NewPlayer _returnvalue)
          (if (== (`self.CurrentPleyerCount`) (`self.MaxPlayerCount`))
            (`KismetSystemLibrary.PrintString` "Game Started")
            (`KismetSystemLibrary.Delay` 10.0)
            (`self.StartPlay`)))))))

(fn `LevelCreate`
  (params (NumPlayers :type Integer))
  (`|SpawnActorFromClass` "/Game/Blueprints/B_CheckBlockLines.B_CheckBlockLines_C" (`KismetMathLibrary.MakeTransform` (0.0 0.0 0.0)) "Undefined" "MultiplyWithRoot" null NumPlayers null))

(fn `UserConstructionScript`)